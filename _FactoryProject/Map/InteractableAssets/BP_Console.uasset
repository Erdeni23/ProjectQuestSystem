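; BP_Console is a quest-driven interactable console that needs power from a linked generator.
; Once powered, interacting during its quest checks the player for a screwdriver; lacking one advances the objective once.
; With one, a one-shot timeline swings the door open, then advances the objective, sparks a brief particle effect and damages the player.
; After a delay it gives the next quest and broadcasts OnConsoleActivated.
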(event `self.ReceiveBeginPlay`
  (add `/Game/_FactoryProject/Map/InteractableAssets/BP_Generator.OnGeneratorActivated` (`self.GeneratorToListenTo`) (delegate `OnGeneratorActivated`)))

(event `OnGeneratorActivated`
  (set `self.HasPower` true))

(event `/Game/_FactoryProject/Map/InteractableAssets/_BPI_Interact.InteractWith`
  (params (Interactor :type "Actor Object Reference") (`ActiveQuestID's` :type "Array of Name (by ref)"))
  (bind (_rotationdoor_roll _rotationdoor_pitch _rotationdoor_yaw) (`KismetMathLibrary.BreakRotator` (`self.RotationDoor`)))
  (if (`/Game/_FactoryProject/ActorComponents/AC_QuestGiverAndProceeder.Is A Part Of Quest?` (`self.AC_QuestGiverAndProceeder`) `ActiveQuestID's`)
    (if (`self.HasPower`)
      (bind _hastools (message `/Game/_FactoryProject/Map/InteractableAssets/_BPI_Interact.CheckForTools` Interactor (`self.Screwdriver`)))
      (if _hastools
        (`/Engine/EditorBlueprintResources/StandardMacros.DoOnce` false
          (:`Completed`
            (set `self.RotationDoor` (`SceneComponent.K2_GetComponentRotation` (`self.Scene`)))
            (bind (_direction _newtrack_0) (`Timeline|Timeline` :!via `PlayFromStart`)
              (:`Update`
                (`SceneComponent.K2_SetWorldRotation` (`self.Scene`) (`KismetMathLibrary.RLerp` (`self.RotationDoor`) (`KismetMathLibrary.MakeRotator` _rotationdoor_roll _rotationdoor_pitch (- _rotationdoor_yaw 130.0)) _newtrack_0) false false))
              (:`Finished`
                (`/Game/_FactoryProject/ActorComponents/AC_QuestGiverAndProceeder.NotifyObjectiveProgress` (`self.AC_QuestGiverAndProceeder`) Interactor)
                (`ActorComponent.Activate` (`self.ParticleSystem`) false)
                (message `/Game/_FactoryProject/Map/InteractableAssets/BPI_MapInterface.DoDamage` Interactor 25.0)
                (`KismetSystemLibrary.Delay` 1.0)
                (`ActorComponent.Deactivate` (`self.ParticleSystem`))
                (`/Game/_FactoryProject/ActorComponents/AC_QuestGiverAndProceeder.GiveQuest` (`self.AC_QuestGiverAndProceeder`) Interactor (`self.NewQuestToGive`))
                (`self.OnConsoleActivated`)))))
        (else
          (`/Engine/EditorBlueprintResources/StandardMacros.DoOnce` false
            (:`Completed`
              (`/Game/_FactoryProject/ActorComponents/AC_QuestGiverAndProceeder.NotifyObjectiveProgress` (`self.AC_QuestGiverAndProceeder`) Interactor))))))))

(fn `CheckForTools`
  (params (RequiredTool :type String))
  (returns (HasTools :type Boolean))
  (return false))

(fn `UserConstructionScript`)