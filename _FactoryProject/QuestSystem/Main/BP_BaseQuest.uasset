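; Base quest that tracks staged objective progress, using the DT_Quests row named by QuestID.
; InitializeQuest and BeginNextStage seed a TargetID-to-count map for the active stage, which UpdateObjectives increments while firing update and completion dispatchers.
; A stage advances when every non-optional objective exactly equals its required amount, and the quest completes after the last stage.
; The objective lookup breaks on first match, preventing updates carrying into the next stage.
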(event `Initialize Quest`
  ;[1 0 0 1 24] Инициализация при создании
  (bind _returnvalue (`|GetDataTableRow` "/Game/_FactoryProject/QuestSystem/Main/DT_Quests.DT_Quests" (`self.QuestID`))
    (:`then`
      (for _array_element (`.Objectives_13_E0F7C3AD45E776D8F481A6BF016E3DEB` (break `/Game/_FactoryProject/QuestSystem/Main/S_StageDetails` (`|GetArrayItem` (`.Stages_16_C01E1FEC40B3750701050795357992D1` (break `/Game/_FactoryProject/QuestSystem/Main/S_QuestDetails` _returnvalue)))))
        (`BlueprintMapLibrary.Map_Add` (`self.CurrentObjectiveProgress`) (`.TargetID_16_18BD3C904395F76734535DA6A89F292F` (break `/Game/_FactoryProject/QuestSystem/Main/S_ObjectiveDetails` _array_element)))))))

(event `UpdateObjectives`
  (params (ObjectiveID :type String) (Amount :type Integer))
  (bind (_value _returnvalue) (`BlueprintMapLibrary.Map_Find` (`self.CurrentObjectiveProgress`) ObjectiveID))
  ;[0.9445 1 0.9725 1 24] Обновляем прогресс текущей задачи
  (if _returnvalue
    (bind (_objective _objectiveindex) (`self.GetCurrentStageObjectiveAndIndex` ObjectiveID)
      (:`true`
        (if (< _value (`.RequiredAmount_17_05725AB741CB2A828EEB219C1FA168C3` (break `/Game/_FactoryProject/QuestSystem/Main/S_ObjectiveDetails` _objective)))
          (`BlueprintMapLibrary.Map_Add` (`self.CurrentObjectiveProgress`) (`.TargetID_16_18BD3C904395F76734535DA6A89F292F` (break `/Game/_FactoryProject/QuestSystem/Main/S_ObjectiveDetails` _objective)) (+ _value Amount))
          (`self.OnCurrentObjectiveUpdated`)
          ;[0.0356 0 1 1 24] Текущая задача выполнена?
          (if (>= (`BlueprintMapLibrary.Map_Find` (`self.CurrentObjectiveProgress`) (`.TargetID_16_18BD3C904395F76734535DA6A89F292F` (break `/Game/_FactoryProject/QuestSystem/Main/S_ObjectiveDetails` _objective))) (`.RequiredAmount_17_05725AB741CB2A828EEB219C1FA168C3` (break `/Game/_FactoryProject/QuestSystem/Main/S_ObjectiveDetails` _objective)))
            (`KismetSystemLibrary.PrintString` null "Задача Выполнена")
            (`self.OnCurrentObjectiveCompleted` _objectiveindex)
            ;[0.0356 0 1 1 24] Стадия выполнена?
            (bind _completed (`self.CheckStageCompeletion`))
            (if _completed
              (`self.OnStageCompleted` (`self.CurrentStage`) self)
              (`/Engine/EditorBlueprintResources/StandardMacros.IncrementInt` (`self.CurrentStage`)
                (:`  `
                  (`BlueprintMapLibrary.Map_Clear` (`self.CurrentObjectiveProgress`))
                  (`KismetSystemLibrary.PrintString` null "Стадия выполнена")
                  (`self.BeginNextStage`
                    (:`Completed`
                      ;[0.0356 0 1 1 24] Квест выполнен?
                      (bind _completed_2 (`self.CheckQuestCompleteion`))
                      (if _completed_2
                        (set `self.IsQuestCompleted` true)
                        (`KismetSystemLibrary.PrintString` null "Квест выполнен")
                        (`self.OnQuestCompleted` self)
                        (else
                          (`KismetSystemLibrary.PrintString` null "Квест ещё не выполнен")))))))
              (else
                (`KismetSystemLibrary.PrintString` null "Стадия ещё не выполнена" true true (struct :`R` 0.94332 :`G` 1.0 :`B` 0.001572 :`A` 1.0))))
            (else
              (`KismetSystemLibrary.PrintString` null "Задача ещё не выполнена")))
          (else
            (`KismetSystemLibrary.PrintString` null "Задача уже выполнена!" true true (struct :`R` 0.94332 :`G` 1.0 :`B` 0.001572 :`A` 1.0))))))
    (else
      (`KismetSystemLibrary.PrintString` null "ФАЛЬШИВКА" true true (struct :`R` 1.0 :`A` 1.0)))))

(fn `CheckQuestCompleteion`
  (returns (Completed :type Boolean))
  (bind _returnvalue (`|GetDataTableRow` "/Game/_FactoryProject/QuestSystem/Main/DT_Quests.DT_Quests" (`self.QuestID`))
    (:`then`
      (return (> (`self.CurrentStage`) (`KismetArrayLibrary.Array_LastIndex` (`.Stages_16_C01E1FEC40B3750701050795357992D1` (break `/Game/_FactoryProject/QuestSystem/Main/S_QuestDetails` _returnvalue))))))))

(fn `CheckStageCompeletion`
  (returns (Completed :type Boolean))
  (bind _returnvalue (`|GetDataTableRow` "/Game/_FactoryProject/QuestSystem/Main/DT_Quests.DT_Quests" (`self.QuestID`))
    (:`then`
      (for _array_element (`.Objectives_13_E0F7C3AD45E776D8F481A6BF016E3DEB` (break `/Game/_FactoryProject/QuestSystem/Main/S_StageDetails` (`|GetArrayItem` (`.Stages_16_C01E1FEC40B3750701050795357992D1` (break `/Game/_FactoryProject/QuestSystem/Main/S_QuestDetails` _returnvalue)) (`self.CurrentStage`))))
        (bind (_description _type _targetid _requiredamount _isoptional) (break `/Game/_FactoryProject/QuestSystem/Main/S_ObjectiveDetails` _array_element))
        (if _isoptional
          _
          (elif (not (== (`BlueprintMapLibrary.Map_Find` (`self.CurrentObjectiveProgress`) _targetid) _requiredamount))
            (return false))))
      (return true))))