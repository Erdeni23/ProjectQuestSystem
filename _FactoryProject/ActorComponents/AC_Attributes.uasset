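; Attributes actor component that tracks health and stamina for its owning actor.
; Damage, heal, consume and restore functions adjust the current values, clamped between zero and their maximums.
; Each change broadcasts the new and maximum values through health or stamina dispatchers.
; Damage also fires a death dispatcher whenever health ends at nearly zero, with no guard against repeat calls.
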(fn `ConsumeStamina`
  (params (ConsumeStaminaAmount :type "Float (double-precision)"))
  (bind _output_get (set `self.CurrentStamina` (`KismetMathLibrary.FClamp` (- (`self.CurrentStamina`) ConsumeStaminaAmount) 0.0 (`self.MaxStamina`))))
  (`self.OnStaminaChanged` _output_get (`self.MaxStamina`)))

(fn `RestoreStamina`
  (params (RestoreStaminaAmount :type "Float (double-precision)"))
  (bind _output_get (set `self.CurrentStamina` (`KismetMathLibrary.FClamp` (+ (`self.CurrentStamina`) RestoreStaminaAmount) 0.0 (`self.MaxStamina`))))
  (`self.OnStaminaChanged` _output_get (`self.MaxStamina`)))

(fn `TakeDamage`
  (params (DamageAmount :type "Float (double-precision)"))
  (bind _output_get (set `self.CurrentHealth` (`KismetMathLibrary.FClamp` (- (`self.CurrentHealth`) DamageAmount) 0.0 (`self.MaxHealth`))))
  (`self.OnHealthChanged` _output_get (`self.MaxHealth`))
  (if (`KismetMathLibrary.NearlyEqual_FloatFloat` _output_get 0.0 0.001)
    (`self.OnDeath`)))

(fn `TakeHeal`
  (params (HealAmount :type "Float (double-precision)"))
  (bind _output_get (set `self.CurrentHealth` (`KismetMathLibrary.FClamp` (+ (`self.CurrentHealth`) HealAmount) 0.0 (`self.MaxHealth`))))
  (`self.OnHealthChanged` _output_get (`self.MaxHealth`)))