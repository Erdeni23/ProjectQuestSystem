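; Player quest manager component that accepts, tracks, updates and completes quests, and drives the quest HUD and pausing journal.
; AddNewQuest validates IDs against DT_Quests, constructs BP_BaseQuest objects and broadcasts acceptance.
; New quests show on the HUD temporarily, reverting to the tracked quest on timeout unless TrackQuest clears the timer.
; Completion events display the finished quest, then after a delay archive its ID, destroy the object and restore the HUD.
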(event `OnQuestWasAddedToActive`
  (params (QuestToTrack :type "/Game/_FactoryProject/QuestSystem/Main/BP_BaseQuest Object Reference"))
  (add `/Game/_FactoryProject/QuestSystem/Main/BP_BaseQuest.OnQuestCompleted` QuestToTrack (delegate `OnQuestCompleted`))
  ;[0.06746 0 1 1 24] Отображение нового квеста на [ShowNewQuestTime] секунд, если игрок его не принял, будет возвращён текущий отслеживаемый квест
  (if (!= (`self.QuestToShow`) (`self.CurrentTrackedQuest`))
    (`KismetSystemLibrary.K2_ClearAndInvalidateTimerHandle` (`self.ShowNewQuest`))
    (bind _returnvalue (`KismetSystemLibrary.K2_SetTimerDelegate` (delegate `NewQuestIgnored`) (`self.ShowNewQuestTime`)))
    (set `self.ShowNewQuest` _returnvalue)
    (`/Game/_FactoryProject/QuestSystem/UI/WBP_HUD_Quest.NewQuestNotificationForPlayer` (`self.CurrentHUDWidget`))))

(event `OnQuestCompleted`
  (params (CompletedQuest :type "/Game/_FactoryProject/QuestSystem/Main/BP_BaseQuest Object Reference"))
  (`self.FinishQuest` CompletedQuest))

(event `NewQuestIgnored`
  ;[0.06746 0 1 1 24] Отображение нового квеста на [ShowNewQuestTime] секунд, если игрок его не принял, будет возвращён текущий отслеживаемый квест
  (`Widget.RemoveFromParent` (`self.CurrentHUDWidget`))
  (`self.Create HUD Widget` (`self.CurrentTrackedQuest`)))

(fn `AddNewQuest`
  (params (QuestID :type Name))
  (`|GetDataTableRow` "/Game/_FactoryProject/QuestSystem/Main/DT_Quests.DT_Quests" QuestID
    (:`then`
      (if (not (`KismetArrayLibrary.Array_IsEmpty` (`self.CurrentActiveQuests`)))
        (for _array_element (`self.CurrentActiveQuests`)
          (bind _questid (`/Game/_FactoryProject/QuestSystem/Main/BP_BaseQuest.QuestID` _array_element))
          (if (== _questid QuestID)
            ;[1 0.9154 0 1 24] Квест уже принят
            (`KismetSystemLibrary.PrintString` (`KismetStringLibrary.Concat_StrStr` (`KismetStringLibrary.Conv_NameToString` _questid) " - Квест уже принят!") true true (struct :`R` 1.0 :`G` 0.989601 :`A` 1.0))
            (return))))
      ;[0 1 0.8205 0.4 24] Принимаем квест - создаем объект BP_BaseQuest - передаем параметр QuestID
      (bind _returnvalue (`|GenericCreateObject` "/Game/_FactoryProject/QuestSystem/Main/BP_BaseQuest.BP_BaseQuest_C" QuestID))
      (`/Game/_FactoryProject/QuestSystem/Main/BP_BaseQuest.Initialize Quest` _returnvalue)
      (`KismetArrayLibrary.Array_AddUnique` (`self.CurrentActiveQuests`) _returnvalue)
      (`KismetSystemLibrary.PrintString` (`KismetStringLibrary.Concat_StrStr` (`KismetStringLibrary.Conv_NameToString` QuestID) " Квест Принят"))
      ;[0 0.2247 1 1 24] Подписчик - Виджет WBP_QuestJournal
      (set `self.QuestToShow` _returnvalue)
      (`self.OnQuestAccepted` _returnvalue)
      (`|ExecutionSequence`
        (:`then_0`
          (`self.Create HUD Widget` _returnvalue)
          (`KismetArrayLibrary.Array_AddUnique` (`self.ActiveQuestID's`) QuestID))
        (:`then_1`
          (`self.OnQuestWasAddedToActive` _returnvalue))
        (:`then_2`
          (return))))
    (:`RowNotFound`
      ;[1 0 0 1 24] Ошибка поиска квеста в DT_Quests
      (`KismetSystemLibrary.PrintString` "Квест не существует, пожалуйста проверьте правильность QuestID у выдающего актора или RowName в DT_Quests" true true (struct :`R` 1.0 :`G` 0.007912 :`A` 1.0) 10.0))))

(fn `AfterQuestCompletionCleanUP`
  (params (CompletedQuest :type "/Game/_FactoryProject/QuestSystem/Main/BP_BaseQuest Object Reference (by ref)"))
  (bind _questid (`/Game/_FactoryProject/QuestSystem/Main/BP_BaseQuest.QuestID` CompletedQuest))
  (set `self.QuestToShow` null)
  ;[0 0 0 1 24] Добавляем в архив, уничтожаем UObject
  (`KismetArrayLibrary.Array_AddUnique` (`self.CompletedQuests`) _questid)
  (`KismetArrayLibrary.Array_RemoveItem` (`self.ActiveQuestID's`) _questid)
  (`KismetArrayLibrary.Array_RemoveItem` (`self.CurrentActiveQuests`) CompletedQuest)
  (`FunctionLibraryCPP.DestroyUObject` CompletedQuest)
  (return))

(fn `CloseJournal`
  (returns (JournalOpened :type Boolean))
  (`Widget.RemoveFromParent` (`self.QuestJournal`))
  (set `PlayerController.bShowMouseCursor` false (`GameplayStatics.GetPlayerController` 0))
  (`GameplayStatics.SetGamePaused` false)
  (`WidgetBlueprintLibrary.SetInputMode_GameOnly` (`GameplayStatics.GetPlayerController` 0))
  (set `self.JournalOpened` false)
  ;[0.0202 0 1 1 24] Возвращаем худ
  (`self.Create HUD Widget` (`self.CurrentTrackedQuest`))
  (return false))

(fn `Create HUD Widget`
  (params (QuestToShow :type "/Game/_FactoryProject/QuestSystem/Main/BP_BaseQuest Object Reference"))
  ;[0 0.2701 1 1 24] Создаём виджет отображения квеста на HUD игрока
  (`/Engine/EditorBlueprintResources/StandardMacros.IsValid` QuestToShow
    (:`Is Valid`
      (`/Engine/EditorBlueprintResources/StandardMacros.IsValid` (`self.CurrentHUDWidget`)
        (:`Is Valid`
          (`Widget.RemoveFromParent` (`self.CurrentHUDWidget`)))
        (:`Is Not Valid`
          _))
      (bind _returnvalue (`|CreateWidget` "/Game/_FactoryProject/QuestSystem/UI/WBP_HUD_Quest.WBP_HUD_Quest_C" null QuestToShow))
      (bind _output_get (set `self.CurrentHUDWidget` _returnvalue))
      (`UserWidget.AddToViewport` _output_get 0)
      (return))))

(fn `IsActiveQuest`
  (params (QuestID :type Name))
  (returns (Active :type Boolean))
  (for _array_element (`self.CurrentActiveQuests`)
    (if (== (`/Game/_FactoryProject/QuestSystem/Main/BP_BaseQuest.QuestID` _array_element) QuestID)
      (return true)))
  (return false))

(fn `OpenJournal`
  (returns (JournalOpened :type Boolean))
  (bind _currenthudwidget (`self.CurrentHUDWidget`))
  ;[1 0 0] Уничтожаем худ чтобы не было оверлапа
  (`/Engine/EditorBlueprintResources/StandardMacros.IsValid` _currenthudwidget
    (:`Is Valid`
      (`Widget.RemoveFromParent` _currenthudwidget))
    (:`Is Not Valid`
      _))
  ;[0 1 0] Создаем виджет журнала и передаем необходимые данные
  (bind _returnvalue (`|CreateWidget` "/Game/_FactoryProject/QuestSystem/UI/WBP_QuestJournal.WBP_QuestJournal_C" (`GameplayStatics.GetPlayerController` 0)))
  (bind _output_get (set `self.QuestJournal` _returnvalue))
  (`UserWidget.AddToViewport` _output_get 0)
  (`WidgetBlueprintLibrary.SetInputMode_GameAndUIEx` (`GameplayStatics.GetPlayerController` 0) _output_get "DoNotLock" false)
  (`/Game/_FactoryProject/QuestSystem/UI/WBP_QuestJournal.OnQuestJournalOpened` (`self.QuestJournal`) (`self.CurrentActiveQuests`) (`self.CurrentTrackedQuest`))
  ;[1 1 1] Пауза на момент открытия журнала
  (set `PlayerController.bShowMouseCursor` true (`GameplayStatics.GetPlayerController` 0))
  (`GameplayStatics.SetGamePaused` true)
  (bind _output_get_2 (set `self.JournalOpened` true))
  (return _output_get_2))

(fn `TrackQuest`
  (params (QuestToTrack :type "/Game/_FactoryProject/QuestSystem/Main/BP_BaseQuest Object Reference"))
  (`/Engine/EditorBlueprintResources/StandardMacros.IsValid` QuestToTrack
    (:`Is Valid`
      (set `self.CurrentTrackedQuest` QuestToTrack)
      (`/Game/_FactoryProject/QuestSystem/UI/WBP_HUD_Quest.BeginTracking` (`self.CurrentHUDWidget`))
      ;[0.05636 0 1] Обнуляем таймер на уничтожение "если квест не был принят", так как квест принят этот таймер не нужен
      (`KismetSystemLibrary.K2_ClearAndInvalidateTimerHandle` (`self.ShowNewQuest`))
      (return))))

(fn `UpdateQuest`
  (params (ObjectiveID :type String) (Amount :type Integer))
  ; Для более корректного отслеживания нужна инвентарная система
  (for _array_element (`self.CurrentActiveQuests`)
    (`/Game/_FactoryProject/QuestSystem/Main/BP_BaseQuest.UpdateObjectives` _array_element ObjectiveID Amount)))