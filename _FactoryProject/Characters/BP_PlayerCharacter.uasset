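; Player character for a first-person-style game with quests, tool collection and health, handling Enhanced Input movement, mouse look and jumping.
; Interaction sphere-traces from the camera and messages actors implementing _BPI_Interact, passing itself and the active quest IDs.
; Quest journal, tracking and progress go to ACQuestManager, damage and healing to ACAttributes, while a Tools array serves as inventory.
; BeginPlay creates the attributes widget and a briefly shown hint.
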(event `self.ReceiveBeginPlay`
  ;[1 0 0.01136 0.5 24] BeginPlay
  (`|ExecutionSequence`
    (:`then_0`
      (`self.CreateWidgets`)
      (`self.Hint`))))

(event `self.ReceivePossessed`
  (params (NewController :type "Controller Object Reference"))
  ;[1 0 0 0.5 24] Event Possesed
  (bind _asbp_player_controller (cast `/Game/_FactoryProject/_Core/BP_PlayerController` NewController))
  (bind _returnvalue (pcsubsystem `EnhancedInputLocalPlayerSubsystem` _asbp_player_controller))
  (`/Engine/EditorBlueprintResources/StandardMacros.IsValid` _returnvalue
    (:`Is Valid`
      (`EnhancedInputSubsystemInterface.AddMappingContext` _returnvalue "/Game/_FactoryProject/_Core/Input/IMC_Default.IMC_Default" 0 (struct))
      (`EnhancedInputSubsystemInterface.AddMappingContext` _returnvalue "/Game/_FactoryProject/_Core/Input/IMC_MouseLook.IMC_MouseLook" 1 (struct)))))

(event `EnhancedInput|/Game/_FactoryProject/_Core/Input/Action/IA_Jump`
  (params (ActionValue :type Boolean) (ElapsedSeconds :type "Float (double-precision)") (TriggeredSeconds :type "Float (double-precision)") (InputAction :type "InputAction Object Reference" :default "/Game/_FactoryProject/_Core/Input/Action/IA_Jump.IA_Jump"))
  ;[0.000439 0.008641 1 0.5 24] Прыжок
  (:`Started`
    (`self.Jump`))
  (:`Completed`
    (`self.StopJumping`)))

(event `EnhancedInput|/Game/_FactoryProject/_Core/Input/Action/IA_MouseLook`
  (params (ActionValue :type "Vector2D Structure") (ElapsedSeconds :type "Float (double-precision)") (TriggeredSeconds :type "Float (double-precision)") (InputAction :type "InputAction Object Reference" :default "/Game/_FactoryProject/_Core/Input/Action/IA_MouseLook.IA_MouseLook"))
  ;[0 0 1 0.5 24] Взгляд
  (:`Triggered`
    (`self.AddControllerYawInput` ActionValue_X)
    (`self.AddControllerPitchInput` ActionValue_Y)))

(event `Key|J` :paused true
  (params (Key :type "Key Structure"))
  (bind _ac_questmanager (`self.AC_QuestManager`))
  ;[0 0 1 1 24] Открыть журнал. J - можно нажимать во время паузы
  (:`Pressed`
    (if (not (`/Game/_FactoryProject/ActorComponents/AC_PlayerQuestManager.JournalOpened` (`self.AC_QuestManager`)))
      (`/Game/_FactoryProject/ActorComponents/AC_PlayerQuestManager.OpenJournal` _ac_questmanager)
      (else
        (`/Game/_FactoryProject/ActorComponents/AC_PlayerQuestManager.CloseJournal` _ac_questmanager :!label _label)))))

(event `Key|Escape` :paused true
  (params (Key :type "Key Structure"))
  ;[0 0 1 1 24] Открыть журнал. J - можно нажимать во время паузы
  (:`Pressed`
    (goto _label)))

(event `EnhancedInput|/Game/_FactoryProject/_Core/Input/Action/IA_Interact`
  (params (ActionValue :type Boolean) (ElapsedSeconds :type "Float (double-precision)") (TriggeredSeconds :type "Float (double-precision)") (InputAction :type "InputAction Object Reference" :default "/Game/_FactoryProject/_Core/Input/Action/IA_Interact.IA_Interact"))
  ;[0 0 1 0.5 24] Взаимодейтсвие, проверка на реализацию интерфейса InteractInterface
  (:`Started`
    (`self.PlayerInteract`)))

(event `EnhancedInput|/Game/_FactoryProject/_Core/Input/Action/IA_Move`
  (params (ActionValue :type "Vector2D Structure") (ElapsedSeconds :type "Float (double-precision)") (TriggeredSeconds :type "Float (double-precision)") (InputAction :type "InputAction Object Reference" :default "/Game/_FactoryProject/_Core/Input/Action/IA_Move.IA_Move"))
  ;[0 0 1 0.5 24] Передвижение
  (:`Triggered`
    (`self.AddMovementInput` (`self.GetActorRightVector`) ActionValue_X)
    (`self.AddMovementInput` (`self.GetActorForwardVector`) ActionValue_Y)))

(event `Key|V`
  (params (Key :type "Key Structure"))
  (bind _ac_questmanager (`self.AC_QuestManager`))
  ;[0 0 1 1 24] Отслеживать отображаемый (новый) квест
  (:`Pressed`
    (`/Game/_FactoryProject/ActorComponents/AC_PlayerQuestManager.TrackQuest` _ac_questmanager (`/Game/_FactoryProject/ActorComponents/AC_PlayerQuestManager.QuestToShow` _ac_questmanager))))

(event `/Game/_FactoryProject/Map/InteractableAssets/_BPI_Interact.AddToolToPlayerInventory`
  (params (ToolToAdd :type String))
  ;[0 1 0 1 24] Добавление инструмента(отвёртка, дрель, молоток и т.д.) в массив инструментов(инвентарь)
  (for _array_element (`self.Tools`)
    (if (`KismetStringLibrary.NotEqual_StrStr` _array_element ToolToAdd)
      (`KismetArrayLibrary.Array_Add` (`self.Tools`) ToolToAdd))))

(event `/Game/_FactoryProject/QuestSystem/BPI_QuestInterface.AddQuest`
  (params (QuestID :type Name))
  ;[0 1 0 1 24] Добавление квеста
  (`/Game/_FactoryProject/ActorComponents/AC_PlayerQuestManager.AddNewQuest` (`self.AC_QuestManager`) QuestID))

(event `/Game/_FactoryProject/QuestSystem/BPI_QuestInterface.UpdateObjectiveProgress`
  (params (ObjectiveID :type String) (Amount :type Integer))
  ;[0 1 0 1 24] Обновление статуса квеста
  (`/Game/_FactoryProject/ActorComponents/AC_PlayerQuestManager.UpdateQuest` (`self.AC_QuestManager`) ObjectiveID Amount))

(event `/Game/_FactoryProject/Map/InteractableAssets/BPI_MapInterface.DoDamage`
  (params (Damage :type "Float (double-precision)"))
  ;[0 1 0.002105] Аттрибуты
  (`/Game/_FactoryProject/ActorComponents/AC_Attributes.TakeDamage` (`self.AC_Attributes`) Damage))

(event `/Game/_FactoryProject/Map/InteractableAssets/BPI_MapInterface.DoHeal`
  (params (HealingAmount :type "Float (double-precision)"))
  ;[0 1 0.002105] Аттрибуты
  (`/Game/_FactoryProject/ActorComponents/AC_Attributes.TakeHeal` (`self.AC_Attributes`) HealingAmount))

(fn `CheckForTools`
  (params (RequiredTool :type String))
  (returns (HasTools :type Boolean))
  (for _array_element (`self.Tools`)
    (if (`KismetStringLibrary.EqualEqual_StrStr` _array_element RequiredTool)
      (return true)))
  (return false))

(fn `CreateWidgets`
  (`|ExecutionSequence`
    (:`then_0`
      (bind _returnvalue (`|CreateWidget` "/Game/_FactoryProject/_Core/UI/HUD/WBP_Attributes.WBP_Attributes_C"))
      (bind _output_get (set `self.Attributes_Widget` _returnvalue))
      (`UserWidget.AddToViewport` _output_get 0))))

(fn `PlayerInteract`
  (bind _camera (`self.Camera`))
  (bind _returnvalue (`SceneComponent.K2_GetComponentLocation` _camera))
  (bind (_outhit _returnvalue_2) (`KismetSystemLibrary.SphereTraceSingle` _returnvalue (+ _returnvalue (* (`SceneComponent.GetForwardVector` _camera) 500.0)) 30.0 "TraceTypeQuery1"))
  (if _returnvalue_2
    (bind (_bblockinghit _binitialoverlap _time _distance _location _impactpoint _normal _impactnormal _physmat _hitactor) (`GameplayStatics.BreakHitResult` _outhit))
    (`/Engine/EditorBlueprintResources/StandardMacros.IsValid` _hitactor
      (:`Is Valid`
        (if (`KismetSystemLibrary.DoesImplementInterface` _hitactor "/Game/_FactoryProject/Map/InteractableAssets/_BPI_Interact._BPI_Interact_C")
          (message `/Game/_FactoryProject/Map/InteractableAssets/_BPI_Interact.InteractWith` _hitactor self (`/Game/_FactoryProject/ActorComponents/AC_PlayerQuestManager.ActiveQuestID's` (`self.AC_QuestManager`))))))))

(fn `UserConstructionScript`)