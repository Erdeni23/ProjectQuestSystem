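; Actor component for the quest system that lets its owner give quests and advance quest objectives.
; GiveQuest and ProgressObjective send interface messages to a target, adding a quest ID or reporting this object's objective ID and quantity.
; IsNedeedQuestIsActive returns true when the object's quest is among the holder's active quests or its row is "_NoQuest".
; CheckPlayersActiveQuests is an empty stub, and the component runs no event logic.
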(fn `CheckPlayersActiveQuests`
  (returns (PlayerActiveQuests :type "Array of Name"))
  (return))

(fn `GiveQuest`
  (params (Target :type "Object Object Reference") (QuestID :type Name))
  (message `/Game/ErdenisQuestSystem/QuestSystem/Framework/BPI_QuestInterface.AddQuest` Target QuestID))

(fn `IsNedeedQuestIsActive`
  (params (QuestHolderReference :type "Object Object Reference"))
  (returns (isActive :type Boolean))
  (bind (_currentquestid_datatable _currentquestid_rowname) (break `DataTableRowHandle` (`self.CurrentQuestID`)))
  (bind (_currentquestid_datatable_2 _currentquestid_rowname_2) (break `DataTableRowHandle` (`self.CurrentQuestID`)))
  ;[0 0 0 0.5] Вернет True если: Нужный квест находится в активных ЛИБО текущий объект не является частью квеста
  (bind _playeractivequests (message `/Game/ErdenisQuestSystem/QuestSystem/Framework/BPI_QuestInterface.CheckPlayersActiveQuests` QuestHolderReference))
  (if (== _currentquestid_rowname "_NoQuest")
    (return true)
    (else
      (for _array_element _playeractivequests
        (if (== _array_element _currentquestid_rowname_2)
          (return true)))
      (return false))))

(fn `ProgressObjective`
  (params (Target :type "Object Object Reference"))
  (message `/Game/ErdenisQuestSystem/QuestSystem/Framework/BPI_QuestInterface.UpdateObjectiveProgress` Target (`self.ThisObjectiveID`) (`self.ThisObjectiveIDQuantity`))
  (return))