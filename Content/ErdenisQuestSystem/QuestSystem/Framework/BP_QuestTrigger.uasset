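; Trigger actor in the quest system that hands out a quest through its ACQuestGiverAndProceeder component, using that component's QuestToGive row name as the ID.
; When player character 0 overlaps the box, it receives the quest and the trigger destroys itself.
; The OnSomethingHappened event instead gives the quest to ActorToGiveQuestTo and leaves the trigger in place.
; CheckPlayersActiveQuests is an empty stub, and an authority check sits unused.
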(event `self.Box.OnComponentBeginOverlap`
  (params (OverlappedComponent :type "PrimitiveComponent Object Reference") (OtherActor :type "Actor Object Reference") (OtherComp :type "PrimitiveComponent Object Reference") (OtherBodyIndex :type Integer) (bFromSweep :type Boolean) (SweepResult :type "HitResult Structure (by ref)"))
  (bind (_questtogive_datatable _questtogive_rowname) (break `DataTableRowHandle` (`/Game/ErdenisQuestSystem/QuestSystem/Framework/AC_QuestGiverAndProceeder.QuestToGive` (`self.AC_QuestGiverAndProceeder`))))
  (if (== OtherActor (`GameplayStatics.GetPlayerCharacter` 0))
    (`/Game/ErdenisQuestSystem/QuestSystem/Framework/AC_QuestGiverAndProceeder.GiveQuest` (`self.AC_QuestGiverAndProceeder`) OtherActor _questtogive_rowname)
    (`self.K2_DestroyActor`)))

(event `OnSomethingHappened`
  (bind (_questtogive_datatable _questtogive_rowname) (break `DataTableRowHandle` (`/Game/ErdenisQuestSystem/QuestSystem/Framework/AC_QuestGiverAndProceeder.QuestToGive` (`self.AC_QuestGiverAndProceeder`))))
  (`/Game/ErdenisQuestSystem/QuestSystem/Framework/AC_QuestGiverAndProceeder.GiveQuest` (`self.AC_QuestGiverAndProceeder`) (`self.ActorToGiveQuestTo`) _questtogive_rowname))

(fn `CheckPlayersActiveQuests`
  (returns (PlayerActiveQuests :type "Array of Name"))
  (return))

(fn `UserConstructionScript`)